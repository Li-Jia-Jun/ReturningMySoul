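; Player controller that lets the player jump possession between pawns registered as accessible for interaction.
; An input possesses the first pawn found in the level, and three more possess entries in PawnArray, maintained through add/remove functions.
; DoPossess manually notifies both BP_InteractComponents and resets the array to just the previous pawn.
; Temporary helpers print the accessible count each tick and restart the level on input.
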(event `InputAction|SwitchCamera`
  (params (Key :type "Key Structure"))
  ;[1 1 1] Start the first possess
  (:`Pressed`
    (bind _outactors (`GameplayStatics.GetAllActorsOfClass` "/Script/Engine.Pawn"))
    (`self.Possess` (`|GetArrayItem` _outactors))))

(event `InputAction|SwitchPossess`
  (params (Key :type "Key Structure"))
  ;[1 1 1] Switch possess
  (:`Pressed`
    (`self.DoPossess` 0)))

(event `InputAction|SwitchPossess2`
  (params (Key :type "Key Structure"))
  ;[1 1 1] Switch possess
  (:`Pressed`
    (`self.DoPossess` 1)))

(event `InputAction|SwitchPossess3`
  (params (Key :type "Key Structure"))
  ;[1 1 1] Switch possess
  (:`Pressed`
    (`self.DoPossess` 2)))

(event `self.ReceiveTick`
  (params (DeltaSeconds :type "Float (single-precision)"))
  ;[1 1 1] Debug: output the current interact objects number player can assess to
  (`KismetSystemLibrary.PrintString` (`KismetStringLibrary.Concat_StrStr` "accessible obj num: " (`KismetStringLibrary.Conv_IntToString` (`KismetArrayLibrary.Array_Length` (`self.PawnArray`)))) true false (struct :`G` 0.66 :`B` 1.0 :`A` 1.0) 0.0))

(event `self.ReceiveBeginPlay`
  ;[1 1 1] Temp: restart current level
  (bind _returnvalue (`GameplayStatics.GetCurrentLevelName` true))
  (set `self.TmpLevelName` _returnvalue))

(event `InputAction|RestartGame`
  (params (Key :type "Key Structure"))
  ;[1 1 1] Temp: restart current level
  (:`Pressed`
    (`GameplayStatics.OpenLevel` (`KismetStringLibrary.Conv_StringToName` (`self.TmpLevelName`)))))

(fn `AddInteractPawn`
  (params (Pawn :type "Pawn Object Reference"))
  (`KismetArrayLibrary.Array_AddUnique` (`self.PawnArray`) Pawn))

(fn `DoPossess`
  (params (whichone :type Integer))
  (locals (OldInteractComponent_ref :type "/Game/ReturnMySoulBP/Blueprints/BP_InteractComponent Object Reference"))
  (bind _pawnarray (`self.PawnArray`))
  (bind _oldinteractcomponent_ref (`local.OldInteractComponent_ref`))
  (bind _output (`|GetArrayItem` _pawnarray whichone))
  ;[1 1 1] Possess the first pawn in array
  (if (> (`KismetArrayLibrary.Array_Length` (`self.PawnArray`)) whichone)
    (set `local.OldInteractComponent_ref` (`self.GetComponentByClass` (`self.K2_GetPawn`) "/Game/ReturnMySoulBP/Blueprints/BP_InteractComponent.BP_InteractComponent_C"))
    (`self.Possess` _output)
    ;[1 1 1] Manually call new pawn possessed event
    (`/Game/ReturnMySoulBP/Blueprints/BP_InteractComponent.OnPlayerPossessed` (`self.GetComponentByClass` _output "/Game/ReturnMySoulBP/Blueprints/BP_InteractComponent.BP_InteractComponent_C"))
    ;[1 1 1] Add old pawn and remove new pawn from player controller
    (`KismetArrayLibrary.Array_Clear` _pawnarray)
    (bind _aspawn (cast `Pawn` (`ActorComponent.GetOwner` _oldinteractcomponent_ref)))
    (`KismetArrayLibrary.Array_Add` _pawnarray _aspawn)
    ;[1 1 1] Manually call old pawn unpossessed
    (`/Game/ReturnMySoulBP/Blueprints/BP_InteractComponent.OnPlayerUnpossessed` _oldinteractcomponent_ref)))

(fn `RemoveInteractPawn`
  (params (Pawn :type "Pawn Object Reference"))
  (`KismetArrayLibrary.Array_RemoveItem` (`self.PawnArray`) Pawn))

(fn `UserConstructionScript`)