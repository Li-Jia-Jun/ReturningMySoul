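; BP_LightSwitch is a light switch that toggles a spotlight when the E key is pressed.
; Each press checks the On flag, flips it, tilts or resets the switch mesh's relative rotation, and shows or hides the SpotLight to match.
; The key event is handled directly in the Blueprint, with no overlap, range or line-of-sight check.
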(event `Key|E`
  (params (Key :type "Key Structure"))
  (bind _lightswitch_switch_002 (`self.lightswitch_Switch_002`))
  (:`Pressed`
    (if (`self.on`)
      (`SceneComponent.K2_SetRelativeRotation` :`self` _lightswitch_switch_002)
      (set `self.on` false)
      (`SceneComponent.SetVisibility` (`self.SpotLight`) false false)
      (else
        (`SceneComponent.K2_SetRelativeRotation` _lightswitch_switch_002 (struct :`Pitch` -10.0) false false)
        (set `self.on` true)
        (`SceneComponent.SetVisibility` (`self.SpotLight`) true false)))))

(fn `UserConstructionScript`)