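; BP_Broom is a possessable broom that the player tilts with the MoveRight input axis.
; The axis adds local roll to the Scene component, then clamps its relative roll between 0 and 70 degrees.
; BeginPlay binds EnablePhysics to BPInteractComponent's possessed event, but that handler is empty.
; The physics toggles, unpossess binding and older force-based movement are disconnected and never run.
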(event `self.ReceiveBeginPlay`
  (add `/Game/ReturnMySoulBP/Blueprints/BP_InteractComponent.PlayerPossessedEvent` (`self.BP_InteractComponent`) (delegate `EnablePhysics`)))

(event `EnablePhysics`
  ;[1 1 1] Simulate Physics when being possessed
)

(event `DisablePhysics`
  ;[1 1 1] Disable Physics when unpossessed
)

(event `InputAxis|MoveRight`
  (params (AxisValue :type "Float (single-precision)"))
  (bind _scene (`self.Scene`))
  ;[1 1 1] Move (rotation only)
  (`SceneComponent.K2_AddLocalRotation` _scene (`KismetMathLibrary.MakeRotator` AxisValue) false false)
  (`SceneComponent.K2_SetRelativeRotation` _scene (`KismetMathLibrary.MakeRotator` (`KismetMathLibrary.FClamp` (.roll (`SceneComponent.RelativeRotation` _scene)) 0.0 70.0) (.pitch (`SceneComponent.RelativeRotation` _scene)) (.yaw (`SceneComponent.RelativeRotation` _scene))) false false))

(fn `UserConstructionScript`)