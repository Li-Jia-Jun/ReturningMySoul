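; Interactive drawer cabinet that the player possesses through BPInteractComponent to slide individual drawers in and out.
; On BeginPlay it gathers the cabinet mesh's child static meshes and selection-sorts them by object name for a stable order.
; Up/Down inputs pick the current drawer, highlighted via custom depth, while Left/Right slide it by StepSize within per-drawer step limits.
; Possess and unpossess events reset the highlights.
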(event `self.ReceiveBeginPlay`
  (bind _bp_interactcomponent (`self.BP_InteractComponent`))
  (`|ExecutionSequence`
    (:`then_0`
      ;[1 1 1] Collect drawer reference
      (for _array_element (`SceneComponent.GetChildrenComponents` (`self.SM_Cabinet`) false)
        (bind _asstatic_mesh_component (cast `StaticMeshComponent` _array_element))
        (`KismetArrayLibrary.Array_Add` (`self.drawers`) _asstatic_mesh_component)
        (`KismetArrayLibrary.Array_Add` (`self.drawerStates`)))
      (`self.SortDrawerArray`))
    (:`then_1`
      ;[1 1 1] Bind event
      (add `/Game/ReturnMySoulBP/Blueprints/BP_InteractComponent.PlayerPossessedEvent` _bp_interactcomponent (delegate `OnPlayerPossessed`))
      (add `/Game/ReturnMySoulBP/Blueprints/BP_InteractComponent.PlayerUnpossessedEvent` _bp_interactcomponent (delegate `OnPlayerUnPossessed`)))))

(event `OnPlayerPossessed`
  ;[1 1 1] Bind event
  (`self.OnPlayerPossess`))

(event `OnPlayerUnPossessed`
  ;[1 1 1] Bind event
  (`self.OnPlayerUnpossess`))

(event `InputAction|Action_Up`
  (params (Key :type "Key Structure"))
  ;[1 1 1] Input
  (:`Pressed`
    (`self.SetCurrentDrawer` (`KismetMathLibrary.Clamp` (+ (`self.CurrentDrawer`) 1) 0 (- (`KismetArrayLibrary.Array_Length` (`self.drawers`)) 1)))))

(event `InputAction|Action_Down`
  (params (Key :type "Key Structure"))
  ;[1 1 1] Input
  (:`Pressed`
    (`self.SetCurrentDrawer` (`KismetMathLibrary.Clamp` (- (`self.CurrentDrawer`) 1) 0 (- (`KismetArrayLibrary.Array_Length` (`self.drawers`)) 1)))))

(event `InputAction|Action_Left`
  (params (Key :type "Key Structure"))
  ;[1 1 1] Input
  (:`Pressed`
    (`self.MoveCurrentDrawer` true)))

(event `InputAction|Action_Right`
  (params (Key :type "Key Structure"))
  ;[1 1 1] Input
  (:`Pressed`
    (`self.MoveCurrentDrawer` false)))

(fn `MoveCurrentDrawer`
  (params (isIncrease :type Boolean))
  (if isIncrease
    ;[1 1 1] Current drawer move out
    (if (< (`|GetArrayItem` (`self.drawerStates`) (`self.CurrentDrawer`)) (`self.MaxStep`))
      (`SceneComponent.K2_AddLocalOffset` (`|GetArrayItem` (`self.drawers`) (`self.CurrentDrawer`)) (`KismetMathLibrary.MakeVector` 0.0 (`self.StepSize`)) false false)
      (`KismetArrayLibrary.Array_Set` (`self.drawerStates`) (`self.CurrentDrawer`) (+ (`|GetArrayItem` (`self.drawerStates`) (`self.CurrentDrawer`)) 1)))
    (else
      ;[1 1 1] Current drawer move in
      (if (> (`|GetArrayItem` (`self.drawerStates`) (`self.CurrentDrawer`)) 0)
        (`SceneComponent.K2_AddLocalOffset` (`|GetArrayItem` (`self.drawers`) (`self.CurrentDrawer`)) (`KismetMathLibrary.MakeVector` 0.0 (* -1 (`self.StepSize`))) false false)
        (`KismetArrayLibrary.Array_Set` (`self.drawerStates`) (`self.CurrentDrawer`) (- (`|GetArrayItem` (`self.drawerStates`) (`self.CurrentDrawer`)) 1))))))

(fn `OnPlayerPossess`
  (`PrimitiveComponent.SetRenderCustomDepth` (`self.SM_Cabinet`) false)
  (for _array_element (`self.drawers`)
    (`PrimitiveComponent.SetRenderCustomDepth` _array_element false))
  (`self.SetCurrentDrawer` 0))

(fn `OnPlayerUnpossess`
  (for _array_element (`self.drawers`)
    (`PrimitiveComponent.SetRenderCustomDepth` _array_element false)))

(fn `SetCurrentDrawer`
  (params (WhichOne :type Integer))
  (`|ExecutionSequence`
    (:`then_0`
      ;[1 1 1] Close last render depth
      (`PrimitiveComponent.SetRenderCustomDepth` (`|GetArrayItem` (`self.drawers`) (`self.CurrentDrawer`)) false))
    (:`then_1`
      ;[1 1 1] Enable new render depth
      (`PrimitiveComponent.SetRenderCustomDepth` (`|GetArrayItem` (`self.drawers`) WhichOne) true))
    (:`then_2`
      ;[1 1 1] Update pointer
      (set `self.CurrentDrawer` WhichOne))))

(fn `SortDrawerArray`
  (locals (num :type Integer) (localMaxIndex :type Integer) (tmp :type "StaticMeshComponent Object Reference"))
  (bind _drawers (`self.drawers`))
  (bind _drawers_2 (`self.drawers`))
  (bind _drawers_3 (`self.drawers`))
  (bind _output (`|GetArrayItem` _drawers_3 (- (`local.num`) 1)))
  ;[1 1 1] Selection sort
  (bind _output_get (set `local.num` (`KismetArrayLibrary.Array_Length` (`self.drawers`))))
  (while (> _output_get 1)
    (set `local.localMaxIndex` 0)
    (for (_array_element _array_index) _drawers_2
      (if (and (`LowEntryExtendedStandardLibrary.GreaterStringString` (`KismetSystemLibrary.GetObjectName` _array_element) (`KismetSystemLibrary.GetObjectName` (`|GetArrayItem` _drawers_2 (`local.localMaxIndex`)))) (< _array_index (`local.num`)))
        (set `local.localMaxIndex` _array_index)))
    (`|ExecutionSequence`
      (:`then_0`
        (if (!= (`|GetArrayItem` _drawers_3 (`local.localMaxIndex`)) _output)
          (set `local.tmp` _output)
          (`KismetArrayLibrary.Array_Set` _drawers (- (`local.num`) 1) (`|GetArrayItem` _drawers (`local.localMaxIndex`)))
          (`KismetArrayLibrary.Array_Set` (`self.drawers`) (`local.localMaxIndex`) (`local.tmp`))))
      (:`then_1`
        (set `local.num` (- (`local.num`) 1))))))

(fn `UserConstructionScript`)