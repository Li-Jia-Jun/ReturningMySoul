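; BP_Ball is a ball that rolls under player control through physics torque.
; The MoveRight and MoveForward input axes each add torque to the Ball component, scaled by RollTorque and the axis value.
; Sideways input drives the X axis with an inverted sign, and forward input drives the Y axis.
; The construction script is empty.
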(event `InputAxis|MoveRight`
  (params (AxisValue :type "Float (single-precision)"))
  ;[1 1 1] Roll left/right
  (`PrimitiveComponent.AddTorque` (`self.Ball`) (`KismetMathLibrary.MakeVector` (* (`self.RollTorque`) AxisValue -1.0)) "None" false))

(event `InputAxis|MoveForward`
  (params (AxisValue :type "Float (single-precision)"))
  ;[1 1 1] Roll forwards/backwards
  (`PrimitiveComponent.AddTorque` (`self.Ball`) (`KismetMathLibrary.MakeVector` 0.0 (* (`self.RollTorque`) AxisValue)) "None" false))

(fn `UserConstructionScript`)