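; BP_hint is a trigger actor that shows a two-part, timed text hint to the player the first time something overlaps it.
; The overlap casts player controller 0 to BP_PlayerController and passes both texts and their durations to UpdateFirstPossessText, then plays a 2D sound.
; Displayed and HintPlayed flags guard the text and sound against repeating, and the overlapping actor is not filtered.
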(event `self.ReceiveActorBeginOverlap`
  (params (OtherActor :type "Actor Object Reference"))
  (if (not (`self.displayed`))
    (bind _asbp_player_controller (cast `/Game/ReturnMySoulBP/Blueprints/BP_PlayerController` (`GameplayStatics.GetPlayerController` 0)))
    (`/Game/ReturnMySoulBP/Blueprints/BP_PlayerController.UpdateFirstPossessText` _asbp_player_controller (`self.text1`) (`self.text2`) (`self.time1`) (`self.time2`))
    (set `self.displayed` true)
    (if (not (`self.Hint played`))
      (`GameplayStatics.PlaySound2D` (`self.SoundPlay`) 1.0 1.0 0.0 null null)
      (set `self.Hint played` true))))

(fn `UserConstructionScript`)