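; BP_Picture is a picture prop that falls once when a bullet hits it.
; On begin play it saves the static mesh's world position and rotation.
; When a component carrying the game instance's bullet tag overlaps the collider, a flag blocks retriggering and a timeline interpolates the mesh from its saved transform to a preset fallen position and rotation.
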(event `self.ReceiveBeginPlay`
  ;[1 1 1] Save the initial position and rotation
  (set `self.InitPos` (`SceneComponent.K2_GetComponentLocation` (`self.StaticMesh`)))
  (set `self.InitRot` (`SceneComponent.K2_GetComponentRotation` (`self.StaticMesh`))))

(event `self.Collider.OnComponentBeginOverlap`
  (params (OverlappedComponent :type "PrimitiveComponent Object Reference") (OtherActor :type "Actor Object Reference") (OtherComp :type "PrimitiveComponent Object Reference") (OtherBodyIndex :type Integer) (bFromSweep :type Boolean) (SweepResult :type "HitResult Structure (by ref)"))
  ;[1 1 1] Fall trigger
  (bind _asbp_game_instance (cast `/Game/ReturnMySoulBP/Blueprints/BP_GameInstance` (`GameplayStatics.GetGameInstance`)))
  (if (and (`ActorComponent.ComponentHasTag` OtherComp (`KismetStringLibrary.Conv_StringToName` (`/Game/ReturnMySoulBP/Blueprints/BP_GameInstance.BulletTag` _asbp_game_instance))) (not (`self.isFall`)))
    (set `self.isFall` true)
    (bind (_direction _newtrack_0) (`Timeline|Timeline_Fall` :`NewTime` 1.5)
      (:`Update`
        (`|ExecutionSequence`
          (:`then_0`
            (`SceneComponent.K2_SetWorldLocation` (`self.StaticMesh`) (`KismetMathLibrary.VLerp` (`self.InitPos`) (`self.FallPos`) _newtrack_0) false false))
          (:`then_1`
            (`SceneComponent.K2_SetWorldRotation` (`self.StaticMesh`) (`KismetMathLibrary.RLerp` (`self.InitRot`) (`self.FallRot`) _newtrack_0) false false)))))))

(fn `UserConstructionScript`)