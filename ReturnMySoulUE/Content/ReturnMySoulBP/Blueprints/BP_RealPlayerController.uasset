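; BP_RealPlayerController is a player controller that lets the player switch possession between interactable pawns with the F key.
; Pawns are registered and removed through AddInteractPawn and RemoveInteractPawn, which maintain a unique array.
; DoPossess takes the first pawn, appends the previous one to the array's end, and manually notifies its BP_InteractComponent of unpossession.
; Tick prints the accessible pawn count as debug output.
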(event `Key|F`
  (params (Key :type "Key Structure"))
  ;[1 1 1] Switch possess
  (:`Pressed`
    (`self.DoPossess`)))

(event `self.ReceiveTick`
  (params (DeltaSeconds :type "Float (single-precision)"))
  ;[1 1 1] Debug: output the current interact objects number player can assess to
  (`KismetSystemLibrary.PrintString` (`KismetStringLibrary.Concat_StrStr` "accessible obj num: " (`KismetStringLibrary.Conv_IntToString` (`KismetArrayLibrary.Array_Length` (`self.PawnArray`)))) true false (struct :`G` 0.66 :`B` 1.0 :`A` 1.0) 0.0))

(fn `AddInteractPawn`
  (params (Pawn :type "Pawn Object Reference"))
  (`KismetArrayLibrary.Array_AddUnique` (`self.PawnArray`) Pawn))

(fn `DoPossess`
  (locals (OldInteractComponent_ref :type "/Game/ReturnMySoulBP/Blueprints/BP_InteractComponent Object Reference"))
  (bind _pawnarray (`self.PawnArray`))
  (bind _oldinteractcomponent_ref (`local.OldInteractComponent_ref`))
  ;[1 1 1] Possess the first pawn in array
  (if (> (`KismetArrayLibrary.Array_Length` (`self.PawnArray`)) 0)
    (set `local.OldInteractComponent_ref` (`self.GetComponentByClass` (`self.K2_GetPawn`) "/Game/ReturnMySoulBP/Blueprints/BP_InteractComponent.BP_InteractComponent_C"))
    (`self.Possess` (`|GetArrayItem` _pawnarray))
    ;[1 1 1] Add old pawn and remove new pawn from player controller
    (`KismetArrayLibrary.Array_Remove` _pawnarray)
    (bind _aspawn (cast `Pawn` (`ActorComponent.GetOwner` _oldinteractcomponent_ref)))
    (`KismetArrayLibrary.Array_Add` _pawnarray _aspawn)
    ;[1 1 1] Manually call new pawn player unpossessed
    (`/Game/ReturnMySoulBP/Blueprints/BP_InteractComponent.OnPlayerUnpossessed` _oldinteractcomponent_ref)))

(fn `RemoveInteractPawn`
  (params (Pawn :type "Pawn Object Reference"))
  (`KismetArrayLibrary.Array_RemoveItem` (`self.PawnArray`) Pawn))

(fn `UserConstructionScript`)