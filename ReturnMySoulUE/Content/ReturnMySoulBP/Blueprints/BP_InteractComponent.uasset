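; Pawn component that supports player possession swapping by detecting nearby interactable pawns and highlighting them.
; Binds overlaps on the owner's shapes carrying the GameInstance interact tag, adding or removing overlapped pawns on BP_PlayerController when player-controlled.
; Otherwise, overlaps toggle custom depth stencil highlighting on all owner meshes.
; Possession handlers update the stencil, fire events, play a first-possession sound, and restore or spawn the AI controller on release.
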(event `self.ReceiveBeginPlay`
  (bind _aspawn (cast `Pawn` (`self.GetOwner`)))
  (`|ExecutionSequence`
    (:`then_0`
      (`self.OnStart` _aspawn))
    (:`then_1`
      ;[1 1 1] Bind Collision Detect
      (bind _tag (`self.GetInteractTag`))
      (for _array_element (`Actor.GetComponentsByTag` (`self.Pawn_ref`) "/Script/Engine.ActorComponent" (`KismetStringLibrary.Conv_StringToName` _tag))
        (bind _asshape_component (cast `ShapeComponent` _array_element))
        (add `PrimitiveComponent.OnComponentBeginOverlap` _asshape_component (delegate `ComponentStartOverlap`))
        (add `PrimitiveComponent.OnComponentEndOverlap` _asshape_component (delegate `ComponentEndOverlap`))))))

(event `ComponentEndOverlap`
  (params (OverlappedComponent :type "PrimitiveComponent Object Reference") (OtherActor :type "Actor Object Reference") (OtherComp :type "PrimitiveComponent Object Reference") (OtherBodyIndex :type Integer))
  ;[1 1 1] Bind Collision Detect
  (`self.OnOverlapEnd` OtherActor OtherComp))

(event `ComponentStartOverlap`
  (params (OverlappedComponent :type "PrimitiveComponent Object Reference") (OtherActor :type "Actor Object Reference") (OtherComp :type "PrimitiveComponent Object Reference") (OtherBodyIndex :type Integer) (bFromSweep :type Boolean) (SweepResult :type "HitResult Structure (by ref)"))
  ;[1 1 1] Bind Collision Detect
  (`self.OnOverlapStart` OtherActor OtherComp))

(fn `GetInteractTag`
  (returns (tag :type String))
  (bind _asbp_game_instance (cast `/Game/ReturnMySoulBP/Blueprints/BP_GameInstance` (`GameplayStatics.GetGameInstance`)))
  (return (`/Game/ReturnMySoulBP/Blueprints/BP_GameInstance.InteractTag` _asbp_game_instance)))

(fn `OnOverlapEnd`
  (params (OtherActor :type "Actor Object Reference") (OtherComp :type "ActorComponent Object Reference"))
  ;[1 1 1] Check interact tag of the overlap object
  (bind _tag (`self.GetInteractTag`))
  (if (`self.ComponentHasTag` OtherComp (`KismetStringLibrary.Conv_StringToName` _tag))
    ;[1 1 1] Avoid self collision
    (if (not (== OtherActor (`self.GetOwner`)))
      ;[1 1 1] Remove the overlap object from player controller
      (bind _aspawn (cast `Pawn` OtherActor))
      (bind _asbp_player_controller (cast `/Game/ReturnMySoulBP/Blueprints/BP_PlayerController` (`Pawn.GetController` (`self.Pawn_ref`)))
        (:`then`
          (`/Game/ReturnMySoulBP/Blueprints/BP_PlayerController.RemoveInteractPawn` _asbp_player_controller _aspawn))
        (:`CastFailed`
          ;[1 1 1] Set stencil for highlight
          (`self.SetOwnerMeshCustomDepth` false 1))))))

(fn `OnOverlapStart`
  (params (OtherActor :type "Actor Object Reference") (OtherComp :type "ActorComponent Object Reference"))
  ;[1 1 1] Check interact tag of the overlap object
  (bind _tag (`self.GetInteractTag`))
  (if (`self.ComponentHasTag` OtherComp (`KismetStringLibrary.Conv_StringToName` _tag))
    ;[1 1 1] Avoid self collision
    (if (not (== OtherActor (`self.GetOwner`)))
      ;[1 1 1] Add the overlap object to player controller
      (bind _aspawn (cast `Pawn` OtherActor))
      (bind _asbp_player_controller (cast `/Game/ReturnMySoulBP/Blueprints/BP_PlayerController` (`Pawn.GetController` (`self.Pawn_ref`)))
        (:`then`
          (`/Game/ReturnMySoulBP/Blueprints/BP_PlayerController.AddInteractPawn` _asbp_player_controller _aspawn))
        (:`CastFailed`
          ;[1 1 1] Set stencil for highlight
          (`self.SetOwnerMeshCustomDepth` true 1))))))

(fn `OnPlayerPossessed`
  (bind _sound (`self.Sound`))
  (`self.SetOwnerMeshCustomDepth` true)
  (`self.PlayerPossessedEvent`)
  ;[1 1 1] The first time player possessed this pawn
  (if (not (`self.IsPlayerHasPossessed`))
    (set `self.IsPlayerHasPossessed` true)
    (if (`KismetSystemLibrary.IsValid` _sound)
      (`GameplayStatics.PlaySound2D` _sound 1.0 1.0 0.0 null null))))

(fn `OnPlayerUnpossessed`
  (bind _aicontroller_ref (`self.AIController_ref`))
  (bind _pawn_ref (`self.Pawn_ref`))
  (if (`KismetSystemLibrary.IsValid` _aicontroller_ref)
    (`Controller.Possess` _aicontroller_ref _pawn_ref)
    (else
      ;[1 1 1] If AI Controller is empty, spawn one
      (`Pawn.SpawnDefaultController` _pawn_ref)
      (bind _asaicontroller (cast `AIController` (`Pawn.GetController` _pawn_ref)))
      (set `self.AIController_ref` _asaicontroller)))
  (`self.SetOwnerMeshCustomDepth` true 1)
  (`self.PlayerUnpossessedEvent`))

(fn `OnStart`
  (params (Pawn :type "Pawn Object Reference"))
  (locals (TmpController :type "Controller Object Reference"))
  (bind _returnvalue (`Pawn.GetController` Pawn))
  (`|ExecutionSequence`
    (:`then_0`
      (bind _asaicontroller (cast `AIController` _returnvalue)
        (:`then`
          (set `self.AIController_ref` _asaicontroller))
        (:`CastFailed`
          (cast `/Game/ReturnMySoulBP/Blueprints/BP_PlayerController` _returnvalue)
          (`self.OnPlayerPossessed`))))
    (:`then_1`
      ;[1 1 1] Store pawn reference
      (set `self.Pawn_ref` Pawn))))

(fn `SetOwnerMeshCustomDepth`
  (params (enable :type Boolean) (stencil :type Integer))
  (for _array_element (`Actor.K2_GetComponentsByClass` (`self.GetOwner`) "/Script/Engine.MeshComponent")
    (`PrimitiveComponent.SetRenderCustomDepth` _array_element enable)
    (`PrimitiveComponent.SetCustomDepthStencilValue` _array_element stencil)))