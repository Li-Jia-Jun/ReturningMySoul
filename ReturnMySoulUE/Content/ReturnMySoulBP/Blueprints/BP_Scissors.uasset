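; BP_Scissors is a pair of scissors whose two halves open and close with the MoveRight input.
; Each Tick adds the MoveRight value to the yaw of SceneRight and its negation to SceneLeft, so the halves rotate in opposite directions.
; Each yaw is clamped to a mirrored range, which limits the swing and stops the halves short of zero yaw.
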(event `self.ReceiveTick`
  (params (DeltaSeconds :type "Float (single-precision)"))
  (bind _returnvalue (`self.GetInputAxisValue`))
  (bind _scene_left (`self.Scene_Left`))
  (bind _scene_right (`self.Scene_Right`))
  ;[1 1 1] Left part rotate
  (`SceneComponent.K2_SetRelativeRotation` _scene_left (`KismetMathLibrary.MakeRotator` (.roll (`SceneComponent.RelativeRotation` _scene_left)) (.pitch (`SceneComponent.RelativeRotation` _scene_left)) (`KismetMathLibrary.FClamp` (+ (.yaw (`SceneComponent.RelativeRotation` _scene_left)) (* _returnvalue -1.0)) 5.0 36.0)) false false)
  ;[1 1 1] Right part rotate
  (`SceneComponent.K2_SetRelativeRotation` _scene_right (`KismetMathLibrary.MakeRotator` (.roll (`SceneComponent.RelativeRotation` _scene_right)) (.pitch (`SceneComponent.RelativeRotation` _scene_right)) (`KismetMathLibrary.FClamp` (+ (.yaw (`SceneComponent.RelativeRotation` _scene_right)) _returnvalue) -36.0 -5.0)) false false))

(fn `UserConstructionScript`)