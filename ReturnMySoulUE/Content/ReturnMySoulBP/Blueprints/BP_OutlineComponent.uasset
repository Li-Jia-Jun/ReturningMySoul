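; Actor component that toggles an outline on its owner's meshes through custom depth and a fixed stencil value.
; At BeginPlay it binds overlap events on owner shapes tagged with the GameInstance's OutlineTag, plus PlayerController possess and unpossess events.
; Player-controlled ThirdPersonCharacter overlaps enable it, while any overlap end disables it.
; Possessing the character sets it by distance to the owner, and unpossessing clears it.
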(event `self.ReceiveBeginPlay`
  (`|ExecutionSequence`
    (:`then_0`
      ;[1 1 1] Store tag
      (bind _asbp_game_instance (cast `/Game/ReturnMySoulBP/Blueprints/BP_GameInstance` (`GameplayStatics.GetGameInstance`)))
      (set `self.Tag` (`/Game/ReturnMySoulBP/Blueprints/BP_GameInstance.OutlineTag` _asbp_game_instance)))
    (:`then_1`
      ;[1 1 1] Bind Collision Event
      (for _array_element (`Actor.GetComponentsByTag` (`self.GetOwner`) "/Script/Engine.ActorComponent" (`KismetStringLibrary.Conv_StringToName` (`self.Tag`)))
        (bind _asshape_component (cast `ShapeComponent` _array_element))
        (add `PrimitiveComponent.OnComponentBeginOverlap` _asshape_component (delegate `OverlapBegin`))
        (add `PrimitiveComponent.OnComponentEndOverlap` _asshape_component (delegate `OverlapEnd`))))
    (:`then_2`
      ;[1 1 1] Bind Third Person Character Event
      (bind _asbp_player_controller (cast `/Game/ReturnMySoulBP/Blueprints/BP_PlayerController` (`GameplayStatics.GetPlayerController` 0)))
      (add `/Game/ReturnMySoulBP/Blueprints/BP_PlayerController.PossessThirdPersonCharacterEvent` _asbp_player_controller (delegate `PossessThirdPersonCharacter`))
      (add `/Game/ReturnMySoulBP/Blueprints/BP_PlayerController.UnpossessThirdPersonCharacterEvent` _asbp_player_controller (delegate `UnpossessThirdPersonCharacter`)))))

(event `OverlapBegin`
  (params (OverlappedComponent :type "PrimitiveComponent Object Reference") (OtherActor :type "Actor Object Reference") (OtherComp :type "PrimitiveComponent Object Reference") (OtherBodyIndex :type Integer) (bFromSweep :type Boolean) (SweepResult :type "HitResult Structure (by ref)"))
  ;[1 1 1] Bind Collision Event
  (bind _isplayer (`self.CheckIsPlayer` OtherActor))
  (if _isplayer
    (`self.SetMeshCustomDepth` true)
    (`KismetSystemLibrary.PrintString` "1")))

(event `OverlapEnd`
  (params (OverlappedComponent :type "PrimitiveComponent Object Reference") (OtherActor :type "Actor Object Reference") (OtherComp :type "PrimitiveComponent Object Reference") (OtherBodyIndex :type Integer))
  ;[1 1 1] Bind Collision Event
  (`self.CheckIsPlayer` OtherActor)
  (if true
    (`self.SetMeshCustomDepth` false)))

(event `PossessThirdPersonCharacter`
  ;[1 1 1] Bind Third Person Character Event
  (if (< (`KismetMathLibrary.Vector_Distance` (`Actor.K2_GetActorLocation` (`Controller.K2_GetPawn` (`GameplayStatics.GetPlayerController` 0))) (`Actor.K2_GetActorLocation` (`self.GetOwner`))) 700.0)
    (`self.SetMeshCustomDepth` true)
    (else
      (`self.SetMeshCustomDepth` false))))

(event `UnpossessThirdPersonCharacter`
  ;[1 1 1] Bind Third Person Character Event
  (`self.SetMeshCustomDepth` false))

(fn `CheckIsPlayer`
  (params (Actor :type "Actor Object Reference"))
  (returns (IsPlayer :type Boolean))
  (bind _asthird_person_character (cast `/Game/ThirdPersonBP/Blueprints/ThirdPersonCharacter` Actor)
    (:`then`
      (cast `/Game/ReturnMySoulBP/Blueprints/BP_PlayerController` (`Pawn.GetController` _asthird_person_character)
        (:`then`
          (return true))
        (:`CastFailed`
          _)))
    (:`CastFailed`
      _))
  (return false))

(fn `SetMeshCustomDepth`
  (params (Enable :type Boolean))
  (for _array_element (`Actor.K2_GetComponentsByClass` (`self.GetOwner`) "/Script/Engine.MeshComponent")
    (`PrimitiveComponent.SetRenderCustomDepth` _array_element Enable)
    (`PrimitiveComponent.SetCustomDepthStencilValue` _array_element 2)))